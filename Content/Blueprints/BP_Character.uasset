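; BP_Character is a character that moves at a set speed, takes damage and destroys itself when health runs out.
; BeginPlay adds a BP_Health widget to the viewport and enables the mouse cursor and click events.
; Tick offsets the MergedChar component by Speed each frame, without sweep or delta-time scaling.
; AnyDamage subtracts from Health via a string-to-int conversion and destroys the actor at zero or below.
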(event EventBeginPlay
  (bind _returnvalue (Game|GetPlayerController 0))
  (bind _returnvalue_2 (UserInterface|CreateWidget "/Game/UI/BP_Health.BP_Health_C" _returnvalue))
  (UserInterface|Viewport|AddtoViewport _returnvalue_2 0)
  (Variables|/Script/Engine.PlayerController|SetbShowMouseCursor _returnvalue true)
  (Variables|/Script/Engine.PlayerController|SetbEnableClickEvents _returnvalue true))

(event EventTick
  (params (DeltaSeconds :type Float%20%28single-precision%29))
  (Transformation|SetWorldLocation (Variables|Default|GetMergedChar) (+ (Variables|Default|GetSpeed) (Transformation|GetWorldLocation (Variables|Default|GetMergedChar))) false false))

(event Game|Damage|EventAnyDamage
  (params (Damage :type Float%20%28single-precision%29) (DamageType :type Damage%20Type%20Object%20Reference) (InstigatedBy :type Controller%20Object%20Reference) (DamageCauser :type Actor%20Object%20Reference))
  (bind _output_get (Variables|Default|SetHealth (Math|Conversions|ToInteger(Byte) (Utilities|String|ToString(Float) (- (Variables|Default|GetHealth) Damage)))))
  (if (<= _output_get 0)
    (Actor|DestroyActor)))

(fn ConstructionScript)